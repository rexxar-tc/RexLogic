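; Buildable logic cable component that delays logic signals by a time set through its own input, active only once placed.
; The top input (Lgk3) sets the delay in milliseconds, clamped to one 60Hz frame because faster logic is unreliable.
; After the delay it calls OverrideLogicPassedIn, temporarily tagging Lgk3 as Disabled so the delay input is excluded during that call.
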(event EventLogicPassedin
  (params (Box :type String) (New%20Logic :type String))
  (bind _lgk3 (Variables|Default|GetLgk3))
  (bind _componenttags (Variables|/Script/Engine.ActorComponent|GetComponentTags _lgk3))
  (if (Variables|Default|GetPlacedDown?)
    (if (Utilities|Enum|Equal(Enum) Box "Lgk3")
      (Variables|Default|SetDelay (/ (Math|Float|Max(Float) (Math|Conversions|ToFloat(Integer) New%20Logic) 16.667) 1e+03)) ; Exec connection to Delay here resets timer when delay changed
    )
    (Utilities|FlowControl|Delay (Variables|Default|GetDelay))
    (bind _returnvalue (Utilities|Array|Add _componenttags "Disabled"))
    (CallFunction|OverrideLogicPassedin Box New%20Logic)
    (Utilities|Array|RemoveIndex _componenttags _returnvalue)))

(fn ConstructionScript
  (|CallParentFunction))