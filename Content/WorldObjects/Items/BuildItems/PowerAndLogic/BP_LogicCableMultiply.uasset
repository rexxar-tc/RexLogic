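; BP_LogicCableMultiply is a logic cable build item that outputs the product of two logic values.
; When logic arrives on any box other than Lgk3, it converts the Logic and LogicB strings to integers and multiplies them.
; It line-traces from Lgk3 and passes the product, as a string, to whatever it hits.
; Skipping Lgk3 as a trigger keeps that box output-only.
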(event EventBeginPlay)

(event Collision|EventActorBeginOverlap
  (params (OtherActor :type Actor%20Object%20Reference)))

(event EventTick
  (params (DeltaSeconds :type Float%20%28single-precision%29)))

(event EventOverrideLogicPassedin
  (params (Box :type String) (New%20Logic :type String))
  (if (not (Utilities|Enum|Equal(Enum) Box "Lgk3"))
    (bind (_hit_actor _hit_box _trace_end) (CallFunction|LogicLineTrace (Variables|Default|GetLgk3)))
    (CallFunction|TryPassLogic _hit_actor _hit_box _trace_end (Utilities|String|ToString(Integer) (* (Math|Conversions|ToInteger(Byte) (Variables|Default|GetLogic)) (Math|Conversions|ToInteger(Byte) (Variables|Default|GetLogicB)))))))

(fn ConstructionScript
  (|CallParentFunction))